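; BP_CrossRoadGameMode is the game mode that runs the HUD, player respawning and the win screen.
; On begin play it creates the game HUD widget and adds it to the viewport.
; Player death destroys the actor, increments the death count shown on the HUD and spawns a new player at a fixed location.
; A win event tells the HUD to show its end screen.
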(event `self.ReceiveBeginPlay`
  (bind _returnvalue (`|CreateWidget` "/Game/Blueprints/BP_GameHUD.BP_GameHUD_C"))
  (bind _output_get (set `self.GameHUDRef` _returnvalue))
  (`UserWidget.AddToViewport` _output_get 0))

(event `self.PlayerDeath`
  (params (Player :type "Car Object Reference"))
  (`self.K2_DestroyActor` Player)
  (bind _result (`/Engine/EditorBlueprintResources/StandardMacros.IncrementInt` (`self.PlayerDeaths`))
    (:`  `
      (`GameHUD.UpdatePlayerDeaths` (`self.GameHUDRef`) _result)
      (`|SpawnActorFromClass` "/Game/Blueprints/BP_Player.BP_Player_C" (`KismetMathLibrary.MakeTransform` (170.0 -10.0 42.0)) "Undefined" "OverrideRootScale" null null))))

(event `self.PlayerWin`
  (`GameHUD.EndScreen` (`self.GameHUDRef`)))

(fn `UserConstructionScript`)