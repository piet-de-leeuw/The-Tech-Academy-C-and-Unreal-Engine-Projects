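; BP_Player is the player actor in a road-crossing game, which dies when it touches a car and wins when it reaches a goal.
; The UpDown axis sets the Collider's physics velocity on both X and Y from Speed, while LeftRight is unimplemented.
; Overlaps with BP_Car or Goal report death or victory to the cached CrossRoadGameMode.
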(event `self.ReceiveBeginPlay`
  (bind _ascross_road_game_mode (cast `CrossRoadGameMode` (`GameplayStatics.GetGameMode`)))
  (set `self.GameModeRef` _ascross_road_game_mode))

(event `InputAxis|UpDown`
  (params (AxisValue :type "Float (single-precision)"))
  (bind _speed (`self.speed`))
  (`PrimitiveComponent.SetPhysicsLinearVelocity` (`self.Collider`) (`KismetMathLibrary.MakeVector` (* AxisValue _speed) (* _speed (stale `InputAxis|LeftRight` AxisValue))) false "None"))

(event `InputAxis|LeftRight`
  (params (AxisValue :type "Float (single-precision)")))

(event `self.ReceiveActorBeginOverlap`
  (params (OtherActor :type "Actor Object Reference"))
  (cast `/Game/Blueprints/BP_Car` OtherActor
    (:`then`
      (`self.Die`))
    (:`CastFailed`
      (cast `Goal` OtherActor)
      (`CrossRoadGameMode.PlayerWin` (`self.GameModeRef`)))))

(event `self.Die`
  (`CrossRoadGameMode.PlayerDeath` (`self.GameModeRef`) self))

(fn `UserConstructionScript`)