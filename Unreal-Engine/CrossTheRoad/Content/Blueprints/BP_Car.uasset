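; BP_Car is a car actor that shuttles back and forth along the world Y axis, reversing at boundaries.
; BeginPlay sets the initial direction sign from the StartDirectionLeft flag.
; Each Tick drives the Collider's physics linear velocity from that sign times Speed, and overlapping a Boundary actor flips the sign.
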(event `self.ReceiveBeginPlay`
  (if (`self.startDirectionLeft`)
    (set `self.direction` -1)
    (else
      (set `self.direction` 1))))

(event `self.ReceiveActorBeginOverlap`
  (params (OtherActor :type "Actor Object Reference"))
  (cast `Boundary` OtherActor)
  (set `self.direction` (* (`self.direction`) -1)))

(event `self.ReceiveTick`
  (params (DeltaSeconds :type "Float (single-precision)"))
  (`PrimitiveComponent.SetPhysicsLinearVelocity` (`self.Collider`) (`KismetMathLibrary.MakeVector` 0.0 (* (`self.direction`) (`self.speed`))) false "None"))

(fn `UserConstructionScript`)